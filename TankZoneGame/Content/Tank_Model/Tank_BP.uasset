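; Player-drivable tank Blueprint that wires up the tank's aiming, track movement, cameras and health bar.
; BeginPlay hands the barrel and turret to the Aiming component, both tracks to TankMovement, and itself to the HealthBar widget.
; Aim axes rotate GimbalY for yaw and SpringArm for pitch, and an action toggles third- and first-person cameras.
; Driving supports either direct per-track throttles or combined move axes through TankMovement.
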(event EventBeginPlay
  (Class|AimingComponent|Initialise (Variables|Default|GetAiming) (Variables|Default|GetBarrel) (Variables|Default|GetTankTurret))
  (Class|TankMovementComponent|SetTracks (Variables|Default|GetTankMovement) (Variables|Default|GetRightTrack) (Variables|Default|GetLeftTrack))
  (bind _ashealth_bar (Utilities|Casting|CastToHealthBar (UserInterface|GetUserWidgetObject (Variables|Default|GetHealth%20Bar))))
  (Variables|/Game/Tank_Model/HealthBar.HealthBar_C|SetPossessedTank _ashealth_bar self))

(event Input|ActionEvents|InputActionChangeCamera
  (params (Key :type Key%20Structure))
  (:Pressed
    (Components|Activation|ToggleActive (Variables|Default|GetCamera))
    (Components|Activation|ToggleActive (Variables|Default|Get1st%20person%20Camera))))

(event Input|AxisEvents|InputAxisMoveRight
  (params (AxisValue :type Float%20%28single-precision%29))
  (Class|TankMovementComponent|MoveRight (Variables|Default|GetTankMovement) AxisValue))

(event Input|AxisEvents|InputAxisLeftTrackThrottle
  (params (AxisValue :type Float%20%28single-precision%29))
  (Class|TrackComponent|SetThrottle (Variables|Default|GetLeftTrack) AxisValue))

(event Input|AxisEvents|InputAxisRightTrackThrottle
  (params (AxisValue :type Float%20%28single-precision%29))
  (Class|TrackComponent|SetThrottle (Variables|Default|GetRightTrack) AxisValue))

(event Input|AxisEvents|InputAxisAImX
  (params (AxisValue :type Float%20%28single-precision%29))
  (Transformation|AddLocalRotation (Variables|Default|GetGimbalY) (Math|Rotator|MakeRotator 0.0 0.0 AxisValue) false false))

(event Input|AxisEvents|InputAxisAimY
  (params (AxisValue :type Float%20%28single-precision%29))
  (Transformation|AddLocalRotation (Variables|Default|GetSpringArm) (Math|Rotator|MakeRotator 0.0 AxisValue 0.0) false false))

(event Input|AxisEvents|InputAxisMove
  (params (AxisValue :type Float%20%28single-precision%29))
  (Class|TankMovementComponent|MoveDirection (Variables|Default|GetTankMovement) AxisValue))

(fn ConstructionScript)